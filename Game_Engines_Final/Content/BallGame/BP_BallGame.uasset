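; BP_BallGame is a ball-throwing minigame actor that shows the BallThrow widget when its Box is overlapped.
; Tick pitches ProjectileSpawnPos to Angle and drives Delay-based loops that cycle Angle, then Power, through repeating ranges until AngleSet and PowerSet lock them.
; Once both are set, it clears the flags, spawns a scaled-down BP_Projectile at that transform and restarts the angle sweep after a pause.
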(event `self.ReceiveTick`
  (params (DeltaSeconds :type "Float (single-precision)"))
  (bind (_returnvalue_location _returnvalue_rotation) (`KismetMathLibrary.BreakTransform` (`SceneComponent.K2_GetComponentToWorld` (`self.Projectile Spawn Pos`))))
  (`SceneComponent.K2_SetRelativeRotation` (`self.Projectile Spawn Pos`) (`KismetMathLibrary.MakeRotator` 0.0 (`self.Angle`)) false false)
  (if (not (`self.AngleSet`))
    (if (> (`self.Angle`) 59.0) :!label _label
      (set `self.Angle` 30.0)
      (`KismetSystemLibrary.Delay` 0.2)
      (else
        (set `self.Angle` (+ (`self.Angle`) 0.5))
        (if (`self.AngleSet`)
          (if (> (`self.Power`) 99.0) :!label _label_2
            (set `self.Power` 0.0)
            (`KismetSystemLibrary.Delay` 0.2)
            (goto _label_2)
            (else
              (set `self.Power` (+ (`self.Power`) 5.0))
              (if (`self.PowerSet`)
                (set `self.PowerSet` false)
                (set `self.AngleSet` false)
                (`|SpawnActorFromClass` "/Game/BallGame/BP_Projectile.BP_Projectile_C" (`KismetMathLibrary.MakeTransform` _returnvalue_location _returnvalue_rotation (0.1 0.1 0.1)) "AlwaysSpawn" "MultiplyWithRoot" null null)
                (`KismetSystemLibrary.Delay` 1.0)
                (goto _label)
                (else
                  (`KismetSystemLibrary.Delay` 0.2)
                  (goto _label_2)))))
          (else
            (`KismetSystemLibrary.Delay` 0.2)
            (goto _label)))))))

(event `self.Box.OnComponentBeginOverlap`
  (params (OverlappedComponent :type "PrimitiveComponent Object Reference") (OtherActor :type "Actor Object Reference") (OtherComp :type "PrimitiveComponent Object Reference") (OtherBodyIndex :type Integer) (bFromSweep :type Boolean) (SweepResult :type "HitResult Structure (by ref)"))
  (bind _returnvalue (`|CreateWidget` "/Game/Widgets/BallThrow.BallThrow_C" (`GameplayStatics.GetPlayerController` 0)))
  (`UserWidget.AddToViewport` _returnvalue 0))

(fn `UserConstructionScript`)