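; Level 2 light puzzle button in a Lights Out style: overlapping its box toggles it and its four linked neighbours (left, right, up, down).
; Each toggle flips Active, swaps the cylinder between on and off materials, and notifies a Brain object.
; The On/off event toggles without propagating further, while a DoOnce with a short delayed reset debounces overlaps.
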(event `self.ReceiveBeginPlay`
  (bind _cylinder (`self.Cylinder`))
  (if (`self.active`)
    (`PrimitiveComponent.SetMaterial` _cylinder 0 "/Game/Lights/MT_ButtonOn.MT_ButtonOn")
    (else
      (`PrimitiveComponent.SetMaterial` _cylinder 0 "/Game/Lights/MT_ButtonOff.MT_ButtonOff"))))

(event `self.Box.OnComponentBeginOverlap`
  (params (OverlappedComponent :type "PrimitiveComponent Object Reference") (OtherActor :type "Actor Object Reference") (OtherComp :type "PrimitiveComponent Object Reference") (OtherBodyIndex :type Integer) (bFromSweep :type Boolean) (SweepResult :type "HitResult Structure (by ref)"))
  (bind _cylinder (`self.Cylinder`))
  (`/Engine/EditorBlueprintResources/StandardMacros.DoOnce` false :!label _label
    (:`Completed`
      (`self.On/off` (`self.Button_Left`))
      (`self.On/off` (`self.Button_Right`))
      (`self.On/off` (`self.Button_Up`))
      (`self.On/off` (`self.Button_Down`))
      (bind _output_get (set `self.active` (not (`self.active`))))
      (if _output_get
        (`PrimitiveComponent.SetMaterial` _cylinder 0 "/Game/Lights/MT_ButtonOn.MT_ButtonOn")
        (else
          (`PrimitiveComponent.SetMaterial` _cylinder 0 "/Game/Lights/MT_ButtonOff.MT_ButtonOff")))
      (message `/Game/Lights/BP_Interface.On/off` (`self.Brain`))
      (`KismetSystemLibrary.Delay` 0.2)
      (goto _label :!via `Reset`))))

(event `/Game/Lights/BP_Interface.On/off`
  (bind _cylinder (`self.Cylinder`))
  (bind _output_get (set `self.active` (not (`self.active`))))
  (if _output_get
    (`PrimitiveComponent.SetMaterial` _cylinder 0 "/Game/Lights/MT_ButtonOn.MT_ButtonOn")
    (else
      (`PrimitiveComponent.SetMaterial` _cylinder 0 "/Game/Lights/MT_ButtonOff.MT_ButtonOff")))
  (message `/Game/Lights/BP_Interface.On/off` (`self.Brain`)))

(fn `UserConstructionScript`)