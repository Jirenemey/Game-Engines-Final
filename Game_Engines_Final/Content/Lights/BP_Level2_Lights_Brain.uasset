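; BP_Level2_Lights_Brain is the controller for the Level 2 lights puzzle, opening a door once every button is active.
; Its On/off event waits briefly, updates Attempts, then gathers all BP_Level2_Lights_Button actors and counts the active ones.
; When that count equals the button total, it destroys the Door actor and toggles Completed on only the first button found.
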(event EventBeginPlay)

(event Collision|EventActorBeginOverlap
  (params (OtherActor :type Actor%20Object%20Reference)))

(event EventTick
  (params (DeltaSeconds :type Float%20%28single-precision%29)))

(event EventOn/off
  (Utilities|FlowControl|Delay 0.1)
  (Variables|Default|SetAttempts (stale _result))
  (bind _outactors (Actor|GetAllActorsOfClass "/Game/Lights/BP_Level2_Lights_Button.BP_Level2_Lights_Button_C"))
  (Variables|Default|SetButtonCount (Utilities|Array|Length _outactors))
  (Variables|Default|SetButtonsActive 0)
  (for _array_element _outactors
    (if (Variables|/Game/Lights/BP_Level2_Lights_Button.BP_Level2_Lights_Button_C|Getactive _array_element)
      (Math|Integer|IncrementInt (Variables|Default|GetButtonsActive)
        (:%20%20
          (if (== (Variables|Default|GetButtonCount) (Variables|Default|GetButtonsActive))
            (Actor|DestroyActor (Variables|Default|GetDoor))
            (bind _outactors_2 (Actor|GetAllActorsOfClass "/Game/Lights/BP_Level2_Lights_Button.BP_Level2_Lights_Button_C"))
            (Variables|/Game/Lights/BP_Level2_Lights_Button.BP_Level2_Lights_Button_C|Setcompleted (Utilities|Array|Get(acopy) _outactors_2) (not (Variables|/Game/Lights/BP_Level2_Lights_Button.BP_Level2_Lights_Button_C|Getcompleted (Utilities|Array|Get(acopy) _outactors_2))))))))))

(fn ConstructionScript)