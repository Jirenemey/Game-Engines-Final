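; BP_Level2_Lights_Brain is an actor that tracks the state of the light buttons in Level 2.
; Its On/off event waits briefly, gathers every BP_Level2_Lights_Button and counts those whose Active flag is set.
; It compares that count to the total number of buttons, but the all-active branch currently triggers nothing.
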(event `/Game/Actors/BP_Interface.On/off`
  (bind _buttonsactive (`self.ButtonsActive`))
  (`KismetSystemLibrary.Delay` 0.1)
  (bind _outactors (`GameplayStatics.GetAllActorsOfClass` "/Game/Actors/BP_Level2_Lights_Button.BP_Level2_Lights_Button_C"))
  (set `self.ButtonCount` (`KismetArrayLibrary.Array_Length` _outactors))
  (set `self.ButtonsActive` 0)
  (for _array_element _outactors
    (if (`/Game/Actors/BP_Level2_Lights_Button.active` _array_element)
      (`/Engine/EditorBlueprintResources/StandardMacros.IncrementInt` _buttonsactive
        (:`  `
          (if (== (`self.ButtonCount`) _buttonsactive)
            _))))))

(fn `UserConstructionScript`)